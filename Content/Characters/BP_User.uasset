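; BP_User is a base user character that can be hovered, selected and clicked to open its own context menu.
; BeginPlay creates a WBP_UserMenu bound to the character, and a capsule click shows it at the mouse position, with HideUserMenu removing it.
; Cursor hover drives the Highlight component on the mesh, while ToggleWidget sets the selection widget's visibility.
; ReadItem is a placeholder for child overrides that prints an error if called unoverridden.
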(event `self.ReceiveBeginPlay`
  (bind _returnvalue (`|CreateWidget` "/Game/UI/Menus/WBP_UserMenu.WBP_UserMenu_C" null self))
  (set `self.WBP_UserMenu` _returnvalue))

(event `self.CapsuleComponent.OnClicked`
  (params (TouchedComponent :type "PrimitiveComponent Object Reference") (ButtonPressed :type "Key Structure"))
  (bind _wbp_usermenu (`self.WBP_UserMenu`))
  (if (not (`Widget.IsInViewport` _wbp_usermenu))
    (`UserWidget.AddToViewport` _wbp_usermenu 0))
  (bind _returnvalue (`WidgetLayoutLibrary.GetMousePositionOnViewport`))
  (`UserWidget.SetPositionInViewport` _wbp_usermenu _returnvalue false))

(event `self.CapsuleComponent.OnBeginCursorOver`
  (params (TouchedComponent :type "PrimitiveComponent Object Reference"))
  ;[1 1 1] Highlight
  (`HighlightComponent.Highlight` (`self.Highlight`) (`self.Mesh`)))

(event `self.CapsuleComponent.OnEndCursorOver`
  (params (TouchedComponent :type "PrimitiveComponent Object Reference"))
  ;[1 1 1] Highlight
  (`HighlightComponent.EndHighlight` (`self.Highlight`) (`self.Mesh`)))

(event `self.ToggleWidget`
  (params (On :type Boolean))
  (`SceneComponent.SetVisibility` (`self.Widget_Selected`) On false))

(fn `HideUserMenu`
  (bind _wbp_usermenu (`self.WBP_UserMenu`))
  (if (`Widget.IsInViewport` _wbp_usermenu)
    (`Widget.RemoveFromParent` _wbp_usermenu)))

(fn `ReadItem`
  (params (ItemToRead :type "Item Object Reference"))
  (`KismetSystemLibrary.PrintString` "The not overriden BP_User.ReadItem is called!" true true (struct :`R` 1.0 :`A` 1.0) 100.0))

(fn `UserConstructionScript`)