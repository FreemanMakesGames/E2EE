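; Obsolete container item actor that can hold one item and carry an optional lock.
; State is derived from whether its item and lock references are valid, with changes swapping the ItemWidget icon between locked, closed and opened.
; Duplicate spawns a disabled deep copy with duplicated contents and lock, aborting with a debug print if it finds a nested container.
; Invalid release or lock-ID queries also print debug errors.
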(fn `ContainItem`
  (params (Item :type "Item Object Reference"))
  (set `self.ContainedItem` Item)
  (`self.ContainVisually`))

(fn `ContainVisually`
  (`ItemWidget.UpdateImage` (`.ItemWidget` (`self.ItemWidget`)) "/Game/Items/Icons/ContainerIcon_Closed.ContainerIcon_Closed"))

(fn `Duplicate`
  (returns (ReturnValue :type "Item Object Reference"))
  (locals (NewContainer :type "/Game/Items/Blueprints/Obsolete_BP_Container Object Reference"))
  (bind _returnvalue (`|SpawnActorFromClass` "Obsolete_BP_Container_C" (`KismetMathLibrary.MakeTransform` (0.0 0.0 0.0)) "Undefined" "OverrideRootScale" null null))
  (set `local.NewContainer` _returnvalue)
  (bind _isoccupied (`self.IsOccupied`))
  (if _isoccupied
    (cast `/Game/Items/Blueprints/Obsolete_BP_Container` (`self.ContainedItem`)
      (:`then`
        (`KismetSystemLibrary.PrintString` "BP_Container.Duplicate finds itself containing another Container!" true true (struct :`R` 1.0 :`A` 1.0) 100.0)
        (return null))
      (:`CastFailed`
        (bind _returnvalue_2 (`self.Duplicate` (`self.ContainedItem`)))
        (`self.ContainItem` (`local.NewContainer`) _returnvalue_2))))
  (bind _islocked (`self.IsLocked`))
  (if _islocked
    (bind _returnvalue_3 (`self.Duplicate` (`self.Lock`)))
    (bind _asobsolete_bp_lock (cast `/Game/Items/Blueprints/Obsolete_BP_Lock` _returnvalue_3))
    (`self.SetLock` (`local.NewContainer`) _asobsolete_bp_lock))
  (`GameUtilities.DisableActor` (`local.NewContainer`))
  (return (`local.NewContainer`)))

(fn `GetLockID`
  (returns (LockID :type Integer))
  (bind _islocked (`self.IsLocked`))
  (if _islocked
    (return (`/Game/Items/Blueprints/Obsolete_BP_Lock.LockID` (`self.Lock`)))
    (else
      (`KismetSystemLibrary.PrintString` "BP_Container.GetLockID is called without checking if it's locked first!" true true (struct :`R` 1.0 :`B` 1.0 :`A` 1.0) 100.0)
      (return -1))))

(fn `IsLocked`
  (returns (IsLocked :type Boolean))
  (return (`KismetSystemLibrary.IsValid` (`self.Lock`))))

(fn `IsOccupied`
  (returns (IsOccupied :type Boolean))
  (return (`KismetSystemLibrary.IsValid` (`self.ContainedItem`))))

(fn `LockVisually`
  (`ItemWidget.UpdateImage` (`.ItemWidget` (`self.ItemWidget`)) "/Game/Items/Icons/ContainerIcon_Locked.ContainerIcon_Locked"))

(fn `OpenVisually`
  (`ItemWidget.UpdateImage` (`.ItemWidget` (`self.ItemWidget`)) "/Game/Items/Icons/ContainerIcon_Opened.ContainerIcon_Opened"))

(fn `ReleaseItem`
  (returns (ReleasedItem :type "Item Object Reference"))
  (locals (ItemToRelease :type "Item Object Reference"))
  (bind _isoccupied (`self.IsOccupied`))
  (if _isoccupied
    (set `local.ItemToRelease` (`self.ContainedItem`))
    (set `self.ContainedItem` null)
    (`self.OpenVisually`)
    (return (`local.ItemToRelease`))
    (else
      (`KismetSystemLibrary.PrintString` "BP_Container.ReleaseItem is called before checking if it's occupied!" true true (struct :`R` 1.0 :`A` 1.0) 100.0))))

(fn `SetLock`
  (params (Lock :type "/Game/Items/Blueprints/Obsolete_BP_Lock Object Reference"))
  (set `self.Lock` Lock)
  (`self.LockVisually`))

(fn `Unlock`
  (set `self.Lock` null)
  (`self.UnlockVisually`))

(fn `UnlockVisually`
  (bind (_itemwidget _itemwidget_2) (`self.ItemWidget`))
  (bind _isoccupied (`self.IsOccupied`))
  (if _isoccupied
    (`ItemWidget.UpdateImage` _itemwidget_2 "/Game/Items/Icons/ContainerIcon_Closed.ContainerIcon_Closed")
    (else
      (`ItemWidget.UpdateImage` _itemwidget_2 "/Game/Items/Icons/ContainerIcon_Opened.ContainerIcon_Opened"))))

(fn `UserConstructionScript`)