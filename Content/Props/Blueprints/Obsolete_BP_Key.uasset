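; Obsolete key prop that acts as an inventory item for unlocking locks and containers.
; It creates its own WBP_Key widget on BeginPlay, forwards widget clicks to its current inventory, and exposes ID, icon, name and an "Unlock" action label.
; Combine delegates to Obsolete_BP_Lock or BP_Container by casting the target, and shows a notification for invalid targets.
; Cursor hover on the mesh toggles its highlight.
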(event `self.ReceiveBeginPlay`
  (bind _returnvalue (`|CreateWidget` "/Game/UI/ItemWidgets/WBP_Key.WBP_Key_C"))
  (bind _output_get (set `self.ItemWidget` _returnvalue))
  (`/Game/UI/ItemWidgets/WBP_Key.Initialize` _output_get self))

(event `/Game/Gameplay/InventorySystem/ItemInterfaces/IBP_Item.SetCurrentInventory`
  (params (CurrentInventory :type "/Game/Gameplay/InventorySystem/BP_InventoryComponent Object Reference"))
  (set `self.CurrentInventory` CurrentInventory))

(event `/Game/Gameplay/InventorySystem/ItemInterfaces/IBP_Combinable.Combine`
  (params (TargetItem :type "/Game/Gameplay/InventorySystem/ItemInterfaces/IBP_Combinable Interface"))
  (if (== (`KismetSystemLibrary.Conv_InterfaceToObject` TargetItem) self)
    (`/Game/Gameplay/BPFuncLib_Utilities.DisplayNotification` "A key can't unlock itself.")
    (else
      (bind _asobsolete_bp_lock (cast `/Game/Props/Blueprints/Obsolete_BP_Lock` TargetItem)
        (:`then`
          ;[1 1 1] Combining with a lock
          (`/Game/Props/Blueprints/Obsolete_BP_Lock.Combine` _asobsolete_bp_lock self))
        (:`CastFailed`
          ;[1 1 1] Combining with a container
          (bind _asbp_container (cast `/Game/Props/Blueprints/BP_Container` TargetItem)
            (:`then`
              (`/Game/Props/Blueprints/BP_Container.Unlock` _asbp_container self))
            (:`CastFailed`
              (`/Game/Gameplay/BPFuncLib_Utilities.DisplayNotification` "Key can't be combined with this item."))))))))

(event `/Game/Gameplay/InventorySystem/ItemInterfaces/IBP_Destroyable.Destroy`
  (`self.K2_DestroyActor`))

(event `self.StaticMesh.OnBeginCursorOver`
  (params (TouchedComponent :type "PrimitiveComponent Object Reference"))
  ;[1 1 1] Highlight
  (`HighlightComponent.Highlight` (`self.Highlight`) (`self.StaticMesh`)))

(event `self.StaticMesh.OnEndCursorOver`
  (params (TouchedComponent :type "PrimitiveComponent Object Reference"))
  ;[1 1 1] Highlight
  (`HighlightComponent.EndHighlight` (`self.Highlight`) (`self.StaticMesh`)))

(fn `GetCombineUsageName`
  (returns (CombineUsageName :type String))
  (return "Unlock"))

(fn `GetCurrentInventory`
  (returns (CurrentInventory :type "/Game/Gameplay/InventorySystem/BP_InventoryComponent Object Reference"))
  (return (`self.CurrentInventory`)))

(fn `GetID`
  (returns (ID :type Integer))
  (return (`self.KeyID`)))

(fn `GetItemIcon`
  (returns (ItemIcon :type "Texture2D Object Reference"))
  (return (`self.ItemIcon`)))

(fn `GetItemName`
  (returns (ItemName :type String))
  (return (`self.ItemName`)))

(fn `GetItemWidget`
  (returns (ItemWidget :type "UserWidget Object Reference"))
  (return (`self.ItemWidget`)))

(fn `HandleItemWidgetOnClicked`
  (`/Game/Gameplay/InventorySystem/BP_InventoryComponent.HandleItemOnClicked` (`self.CurrentInventory`) self))

(fn `UserConstructionScript`)