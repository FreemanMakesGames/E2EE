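; Inventory component that stores items and drives the inventory grid UI and a per-item context menu.
; BeginPlay creates both widgets and derives grid columns, rows and storage from panel size divided by icon size, using a throwaway item widget.
; Adding creates an item widget placed by index; removing the active item clears and rebuilds the grid to work around RemoveChild.
; It also toggles the inventory and positions the menu at the mouse.
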(event `self.ReceiveBeginPlay`
  (`|ExecutionSequence`
    (:`then_0`
      ;[1 1 1] Initialize WBP_Inventory.
      (bind _returnvalue (`|CreateWidget` "/Game/UI/WBP_Inventory.WBP_Inventory_C"))
      (bind _output_get (set `self.WBP_Inventory` _returnvalue))
      ;[1 1 1] Set GridPanelOfItems.
      (set `self.GridPanelOfItems` (`/Game/UI/WBP_Inventory.GridPanel_Items` _output_get)))
    (:`then_1`
      ;[1 1 1] Initialize WBP_ItemMenu
      (bind _returnvalue_2 (`|CreateWidget` "/Game/UI/WBP_ItemMenu.WBP_ItemMenu_C"))
      (bind _output_get_2 (set `self.WBP_ItemMenu` _returnvalue_2))
      (set `/Game/UI/WBP_ItemMenu.MyInventory` self _output_get_2))
    (:`then_2`
      (`self.SetInventoryDimensions`))))

(fn `AddItem`
  (params (NewItem :type "/Game/Gameplay/BP_InventoryItemData Object Reference"))
  (locals (WBP_Item :type "/Game/UI/WBP_Item Object Reference") (ItemIndex :type Integer :default 0))
  (bind _inventorygridmaxcolumns (`self.InventoryGridMaxColumns`))
  (bind _wbp_item (`local.WBP_Item`))
  (bind _newitem (`local.NewItem`))
  (bind _itemindex (`local.ItemIndex`))
  (`|ExecutionSequence`
    (:`then_0`
      ;[1 1 1] Backend array addition
      (bind _returnvalue (`KismetArrayLibrary.Array_Add` (`self.Items`) (`local.NewItem`)))
      (set `local.ItemIndex` _returnvalue))
    (:`then_1`
      ;[1 1 1] Helper set
      (bind _returnvalue_2 (`|CreateWidget` "/Game/UI/WBP_Item.WBP_Item_C"))
      (set `local.WBP_Item` _returnvalue_2))
    (:`then_2`
      ;[1 1 1] Setup WBP_Item.
      (set `/Game/UI/WBP_Item.MyItem` _newitem _wbp_item)
      (set `/Game/UI/WBP_Item.MyInventory` self _wbp_item)
      (`Image.SetBrushFromTexture` (`/Game/UI/WBP_Item.Image_Icon` _wbp_item) (`/Game/Gameplay/BP_InventoryItemData.Icon` _newitem) false)
      ;[1 1 1] WBP_Items array addition
      (`KismetArrayLibrary.Array_Add` (`self.WBP_Items`) (`local.WBP_Item`)))
    (:`then_3`
      ;[1 1 1] Add WBP_Item to grid.
      (bind _returnvalue_3 (`GridPanel.AddChildToGrid` (`self.GridPanelOfItems`) (`local.WBP_Item`)))
      (`GridSlot.SetColumn` _returnvalue_3 (mod _itemindex _inventorygridmaxcolumns))
      (`GridSlot.SetRow` _returnvalue_3 (/ _itemindex _inventorygridmaxcolumns)))))

(fn `CountItems`
  (returns (NumberOfItems :type Integer))
  (return (`KismetArrayLibrary.Array_Length` (`self.Items`))))

(fn `HideItemMenu`
  (`Widget.RemoveFromParent` (`self.WBP_ItemMenu`)))

(fn `RemoveItem`
  (bind _inventorygridmaxcolumns (`self.InventoryGridMaxColumns`))
  (bind _gridpanelofitems (`self.GridPanelOfItems`))
  (`|ExecutionSequence`
    (:`then_0`
      ;[1 1 1] Backend array removal
      (`KismetArrayLibrary.Array_RemoveItem` (`self.Items`) (`/Game/UI/WBP_Item.MyItem` (`self.ActiveWBP_Item`))))
    (:`then_1`
      ;[1 1 1] WBP_Items array removal
      (`KismetArrayLibrary.Array_RemoveItem` (`self.WBP_Items`) (`self.ActiveWBP_Item`)))
    (:`then_2`
      ;[1 1 1] Reset ActiveWBP_Item to nothing.
      (set `self.ActiveWBP_Item` null))
    (:`then_3`
      ;[1 1 1] Clear the grid panel, then re-add, because grid panel's "Remove Child" seems broken.
      (`PanelWidget.ClearChildren` _gridpanelofitems)
      (for (_array_element _array_index) (`self.WBP_Items`)
        (bind _returnvalue (`GridPanel.AddChildToGrid` _gridpanelofitems _array_element))
        (`GridSlot.SetColumn` _returnvalue (mod _array_index _inventorygridmaxcolumns))
        (`GridSlot.SetRow` _returnvalue (/ _array_index _inventorygridmaxcolumns))))))

(fn `SetInventoryDimensions`
  (bind _returnvalue (`|CreateWidget` "/Game/UI/WBP_Item.WBP_Item_C")) ; Very hacky an instance
  (bind (_returnvalue_x _returnvalue_y) (`KismetMathLibrary.BreakVector2D` (/ (`CanvasPanelSlot.GetSize` (`WidgetLayoutLibrary.SlotAsCanvasSlot` (`self.GridPanelOfItems`))) (`.ImageSize` (break `SlateBrush` (`Image.Brush` (`/Game/UI/WBP_Item.Image_Icon` _returnvalue)))))))
  (bind _output_get (set `self.InventoryGridMaxColumns` (`KismetMathLibrary.FTrunc` _returnvalue_x)))
  (bind _output_get_2 (set `self.InventoryGridMaxRows` (`KismetMathLibrary.FTrunc` _returnvalue_y)))
  (set `self.InventoryMaxStorage` (* _output_get_2 _output_get)))

(fn `ShowItemMenu`
  (params (ClickedWBP_Item :type "/Game/UI/WBP_Item Object Reference"))
  (bind _wbp_itemmenu (`self.WBP_ItemMenu`))
  (set `self.ActiveWBP_Item` ClickedWBP_Item)
  (if (not (`Widget.IsInViewport` _wbp_itemmenu))
    (`UserWidget.AddToViewport` _wbp_itemmenu 0))
  (bind _returnvalue (`WidgetLayoutLibrary.GetMousePositionOnViewport`))
  (`UserWidget.SetPositionInViewport` _wbp_itemmenu _returnvalue false))

(fn `ToggleInventory`
  (bind _wbp_itemmenu (`self.WBP_ItemMenu`))
  (if (`Widget.IsInViewport` (`self.WBP_Inventory`))
    (`Widget.RemoveFromParent` (`self.WBP_Inventory`))
    (if (`Widget.IsInViewport` _wbp_itemmenu)
      (`Widget.RemoveFromParent` _wbp_itemmenu))
    (else
      (`UserWidget.AddToViewport` (`self.WBP_Inventory`) 0))))