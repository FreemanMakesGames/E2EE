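; BP_WorkTable is a work table prop with a widget menu for making lock and key pairs and containers.
; On BeginPlay it binds the menu's two buttons to spawn functions that use the table's spawn points.
; Each pair spawns an Obsolete_BP_Lock and BP_Key sharing the E2EEGameStateBase's current pair ID, which is then incremented.
; Only one valid container exists per table, and cursor hover highlights the mesh.
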(event `OnClicked_MakeKeyPairButton`
  (`self.SpawnKeyPair`))

(event `self.ReceiveBeginPlay`
  (bind _aswbp_work_table_menu (cast `/Game/UI/WBP_WorkTableMenu` (`WidgetComponent.GetUserWidgetObject` (`self.Menu`))))
  (set `self.WBP_WorkTableMenu` _aswbp_work_table_menu)
  (`|ExecutionSequence`
    (:`then_0`
      (add `Button.OnClicked` (`/Game/UI/WBP_WorkTableMenu.MakeKeyPairButton` (`self.WBP_WorkTableMenu`)) (delegate `OnClicked_MakeKeyPairButton`)))
    (:`then_1`
      (add `Button.OnClicked` (`/Game/UI/WBP_WorkTableMenu.MakeContainerButton` (`self.WBP_WorkTableMenu`)) (delegate `OnClicked_MakeContainerButton`)))))

(event `OnClicked_MakeContainerButton`
  (`self.SpawnContainer`))

(event `self.StaticMeshComponent.OnBeginCursorOver`
  (params (TouchedComponent :type "PrimitiveComponent Object Reference"))
  ;[1 1 1] Highlight
  (`HighlightComponent.Highlight` (`self.Highlight`) (`self.StaticMeshComponent`)))

(event `self.StaticMeshComponent.OnEndCursorOver`
  (params (TouchedComponent :type "PrimitiveComponent Object Reference"))
  ;[1 1 1] Highlight
  (`HighlightComponent.EndHighlight` (`self.Highlight`) (`self.StaticMeshComponent`)))

(fn `SpawnContainer`
  ;[1 1 1] Check to spawn only 1 container per table.
  (if (not (`KismetSystemLibrary.IsValid` (`self.SpawnedContainer`)))
    (bind _returnvalue (`|SpawnActorFromClass` "/Game/Props/Blueprints/BP_Container.BP_Container_C" (`SceneComponent.K2_GetComponentToWorld` (`self.SpawnPoint_Container`)) "Undefined" "OverrideRootScale" null null))
    (set `self.SpawnedContainer` _returnvalue)))

(fn `SpawnKeyPair`
  (locals (CurrentKeyPairID :type Integer :default 0))
  (bind _ase2eegame_state_base (cast `E2EEGameStateBase` (`GameplayStatics.GetGameState`)))
  (bind _returnvalue (`E2EEGameStateBase.GetCurrentKeyPairID` _ase2eegame_state_base))
  (set `local.CurrentKeyPairID` _returnvalue)
  (`|ExecutionSequence`
    (:`then_0`
      (`|SpawnActorFromClass` "/Game/Props/Blueprints/Obsolete_BP_Lock.Obsolete_BP_Lock_C" (`SceneComponent.K2_GetComponentToWorld` (`self.SpawnPoint_Lock`)) "Undefined" "OverrideRootScale" null (`local.CurrentKeyPairID`) null))
    (:`then_1`
      (`|SpawnActorFromClass` "/Game/Props/Blueprints/BP_Key.BP_Key_C" (`SceneComponent.K2_GetComponentToWorld` (`self.SpawnPoint_Key`)) "Undefined" "OverrideRootScale" null (`local.CurrentKeyPairID`) null))
    (:`then_2`
      (`E2EEGameStateBase.IncrementCurrentKeyPairID` _ase2eegame_state_base))))

(fn `UserConstructionScript`)