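; Player controller Blueprint with an event that toggles an inventory widget.
; If the widget is in the viewport, ToggleInventory removes it from its parent.
; Otherwise it casts the widget to WBP_Inventory and calls AddItem on its TileViewItems, with no add-to-viewport call.
; An InventoryComponent lookup on the active character is present but unused, and the construction script is empty.
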(event `self.ToggleInventory`
  (if (`Widget.IsInViewport` (`self.InventoryWidget`))
    (`Widget.RemoveFromParent` (`self.InventoryWidget`))
    (else
      (bind _aswbp_inventory (cast `/Game/UI/WBP_Inventory` (`self.InventoryWidget`)))
      (`ListView.AddItem` (`/Game/UI/WBP_Inventory.TileView_Items` _aswbp_inventory) null))))

(fn `UserConstructionScript`)