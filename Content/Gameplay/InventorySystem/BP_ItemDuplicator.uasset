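; BP_ItemDuplicator spawns copies of inventory items (locks, keys, containers and messages) and returns each fully disabled.
; DuplicateItem casts the item to its type and calls the matching helper; lock and key copies keep the original ID, while messages spawn with no data copied.
; DuplicateContainer recursively copies the contained item and any engaged lock, but prints an error and returns nothing on finding a nested container.
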(fn `DuplicateContainer`
  (params (OriginalContainer :type "/Game/Items/Blueprints/BP_Container Object Reference"))
  (returns (Clone :type "/Game/Items/Blueprints/BP_Container Object Reference"))
  (locals (NewContainer :type "/Game/Items/Blueprints/BP_Container Object Reference"))
  (bind _originalcontainer (`local.OriginalContainer`))
  (bind _originalcontainer_2 (`local.OriginalContainer`))
  (bind _newcontainer (`local.NewContainer`))
  (bind _containeditem (`/Game/Items/Blueprints/BP_Container.ContainedItem` _originalcontainer_2))
  (bind _returnvalue (`|SpawnActorFromClass` "/Game/Items/Blueprints/BP_Container.BP_Container_C" (`KismetMathLibrary.MakeTransform` (0.0 0.0 0.0)) "Undefined" "OverrideRootScale" null null))
  (set `local.NewContainer` _returnvalue)
  (bind _isoccupied (`/Game/Items/Blueprints/BP_Container.IsOccupied` _originalcontainer_2))
  (if _isoccupied
    (cast `/Game/Items/Blueprints/BP_Container` _containeditem
      (:`then`
        (`KismetSystemLibrary.PrintString` "BP_Inventory.DuplicateItem finds a Container within a Container!!!" true true (struct :`R` 1.0 :`A` 1.0) 100.0)
        (return null))
      (:`CastFailed`
        (bind _clone (`self.DuplicateItem` _containeditem))
        (`/Game/Items/Blueprints/BP_Container.ContainItem` (`local.NewContainer`) _clone))))
  (bind _islocked (`/Game/Items/Blueprints/BP_Container.IsLocked` _originalcontainer))
  (if _islocked
    (bind _clone_2 (`self.DuplicateLock` (`/Game/Items/Blueprints/BP_Container.Lock` _originalcontainer)))
    (`/Game/Items/Blueprints/BP_Container.SetLock` _newcontainer _clone_2))
  (return _newcontainer))

(fn `DuplicateItem`
  (params (ItemToDuplicate :type "Item Object Reference"))
  (returns (Clone :type "Item Object Reference"))
  (bind _asbp_lock (cast `/Game/Items/Blueprints/BP_Lock` ItemToDuplicate)
    (:`then`
      (bind _clone (`self.DuplicateLock` _asbp_lock))
      (`/Game/Gameplay/BPFuncLib_Utilities.CompletelyDisableActorWithPrimitiveComponent` _clone)
      (return _clone))
    (:`CastFailed`
      (bind _asbp_key (cast `/Game/Items/Blueprints/BP_Key` ItemToDuplicate)
        (:`then`
          (bind _clone_2 (`self.DuplicateKey` _asbp_key))
          (`/Game/Gameplay/BPFuncLib_Utilities.CompletelyDisableActorWithPrimitiveComponent` _clone_2)
          (return _clone_2))
        (:`CastFailed`
          (bind _asbp_container (cast `/Game/Items/Blueprints/BP_Container` ItemToDuplicate)
            (:`then`
              (bind _clone_3 (`self.DuplicateContainer` _asbp_container))
              (`/Game/Gameplay/BPFuncLib_Utilities.CompletelyDisableActorWithPrimitiveComponent` _clone_3)
              (return _clone_3))
            (:`CastFailed`
              (bind _asbp_message (cast `/Game/Items/Blueprints/BP_Message` ItemToDuplicate))
              (bind _clone_4 (`self.DuplicateMessage` _asbp_message))
              (`/Game/Gameplay/BPFuncLib_Utilities.CompletelyDisableActorWithPrimitiveComponent` _clone_4)
              (return _clone_4))))))))

(fn `DuplicateKey`
  (params (OriginalKey :type "/Game/Items/Blueprints/BP_Key Object Reference"))
  (returns (Clone :type "/Game/Items/Blueprints/BP_Key Object Reference"))
  (bind _returnvalue (`|SpawnActorFromClass` "/Game/Items/Blueprints/BP_Key.BP_Key_C" (`KismetMathLibrary.MakeTransform` (0.0 0.0 0.0)) "Undefined" "OverrideRootScale" null null))
  (bind _id (`/Game/Items/Blueprints/BP_Key.GetID` OriginalKey))
  (`/Game/Items/Blueprints/BP_Key.SetID` _returnvalue _id)
  (return _returnvalue))

(fn `DuplicateLock`
  (params (OriginalLock :type "/Game/Items/Blueprints/BP_Lock Object Reference"))
  (returns (Clone :type "/Game/Items/Blueprints/BP_Lock Object Reference"))
  (bind _returnvalue (`|SpawnActorFromClass` "/Game/Items/Blueprints/BP_Lock.BP_Lock_C" (`KismetMathLibrary.MakeTransform` (0.0 0.0 0.0)) "Undefined" "OverrideRootScale" null null))
  (bind _id (`/Game/Items/Blueprints/BP_Lock.GetID` OriginalLock))
  (`/Game/Items/Blueprints/BP_Lock.SetID` _returnvalue _id)
  (return _returnvalue))

(fn `DuplicateMessage`
  (params (OriginalMessage :type "/Game/Items/Blueprints/BP_Message Object Reference"))
  (returns (Clone :type "/Game/Items/Blueprints/BP_Message Object Reference"))
  (bind _returnvalue (`|SpawnActorFromClass` "/Game/Items/Blueprints/BP_Message.BP_Message_C" (`KismetMathLibrary.MakeTransform` (0.0 0.0 0.0)) "Undefined" "OverrideRootScale" null null))
  (return _returnvalue))

(fn `UserConstructionScript`)