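; BP_ItemCombiner resolves combining two inventory items, covering lock, key and container pairings.
; CombineItems casts the first item to pick the action and checks the second, showing a notification for invalid pairs.
; Locking stores the lock on an unlocked container; unlocking requires matching key and lock IDs, both updating container visuals.
; Placing an item in a container routes to ContainItem, which is an empty stub.
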(fn `CombineItems`
  (params (Item1 :type "Item Object Reference") (Item2 :type "Item Object Reference"))
  (locals (NewLocalVar_0 :type "Item Object Reference"))
  (bind _item2 (`local.Item2`))
  (bind _asbp_lock (cast `/Game/Items/Blueprints/BP_Lock` Item1)
    (:`then`
      (bind _asbp_container (cast `/Game/Items/Blueprints/BP_Container` (`local.Item2`))
        (:`then`
          (`self.LockContainer` _asbp_lock _asbp_container))
        (:`CastFailed`
          (`/Game/Gameplay/BPFuncLib_Utilities.DisplayNotification` "You can't lock this."))))
    (:`CastFailed`
      (bind _asbp_key (cast `/Game/Items/Blueprints/BP_Key` Item1)
        (:`then`
          (bind _asbp_container_2 (cast `/Game/Items/Blueprints/BP_Container` (`local.Item2`))
            (:`then`
              (`self.UnlockContainer` _asbp_key _asbp_container_2))
            (:`CastFailed`
              (`/Game/Gameplay/BPFuncLib_Utilities.DisplayNotification` "You can't lock this."))))
        (:`CastFailed`
          (bind _asbp_container_3 (cast `/Game/Items/Blueprints/BP_Container` Item1))
          (cast `/Game/Items/Blueprints/BP_Container` _item2
            (:`then`
              (`/Game/Gameplay/BPFuncLib_Utilities.DisplayNotification` "You can't contain another container, sorry!"))
            (:`CastFailed`
              (`self.ContainItem` _asbp_container_3 _item2))))))))

(fn `ContainItem`
  (params (Container :type "/Game/Items/Blueprints/BP_Container Object Reference") (Item :type "Item Object Reference")))

(fn `LockContainer`
  (params (Lock :type "/Game/Items/Blueprints/BP_Lock Object Reference") (Container :type "/Game/Items/Blueprints/BP_Container Object Reference"))
  (bind _container (`local.Container`))
  (if (`KismetSystemLibrary.IsValid` (`/Game/Items/Blueprints/BP_Container.Lock` Container))
    (`/Game/Gameplay/BPFuncLib_Utilities.DisplayNotification` "This container is already locked!")
    (else
      (set `/Game/Items/Blueprints/BP_Container.Lock` (`local.Lock`) _container)
      (`/Game/Items/Blueprints/BP_Container.LockVisually` _container))))

(fn `UnlockContainer`
  (params (Key :type "/Game/Items/Blueprints/BP_Key Object Reference") (Container :type "/Game/Items/Blueprints/BP_Container Object Reference"))
  (locals (TargetLock :type "/Game/Items/Blueprints/BP_Lock Object Reference"))
  (bind _container (`local.Container`))
  (bind _output_get (set `local.TargetLock` (`/Game/Items/Blueprints/BP_Container.Lock` Container)))
  (if (`KismetSystemLibrary.IsValid` _output_get)
    (if (== (`/Game/Items/Blueprints/BP_Lock.LockID` (`local.TargetLock`)) (`/Game/Items/Blueprints/BP_Key.KeyID` (`local.Key`)))
      (set `/Game/Items/Blueprints/BP_Container.Lock` null _container)
      (`/Game/Items/Blueprints/BP_Container.UnlockVisually` _container)
      (else
        (`/Game/Gameplay/BPFuncLib_Utilities.DisplayNotification` "The key doesn't match the lock!")))
    (else
      (`/Game/Gameplay/BPFuncLib_Utilities.DisplayNotification` "This container isn't locked!"))))

(fn `UserConstructionScript`)