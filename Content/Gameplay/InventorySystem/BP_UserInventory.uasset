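; Inventory component for the user that stores items, shows them in a grid widget, and can send them to a Messenger at the current waypoint.
; Capacity comes from grid panel size divided by lock icon size, and items are placed by array index.
; Clicking an item opens a menu at the mouse, or in combine mode combines it with the active item through IBP_Combinable.
; Removal clears and rebuilds the grid to work around RemoveChild.
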(event `self.ReceiveBeginPlay`
  (`|ExecutionSequence`
    (:`then_0`
      ;[1 1 1] Initialize WBP_Inventory.
      (bind _returnvalue (`|CreateWidget` "/Game/UI/WBP_UserInventory.WBP_UserInventory_C" null self))
      (bind _output_get (set `self.InventoryWidget` _returnvalue))
      ;[1 1 1] Set GridPanelOfItems.
      (set `self.GridPanelOfItems` (`/Game/UI/WBP_UserInventory.GridPanel_Items` _output_get)))
    (:`then_1`
      ;[1 1 1] Initialize WBP_ItemMenu
      (bind _returnvalue_2 (`|CreateWidget` "/Game/UI/WBP_ItemMenu.WBP_ItemMenu_C"))
      (bind _output_get_2 (set `self.WBP_ItemMenu` _returnvalue_2))
      (set `/Game/UI/WBP_ItemMenu.MyInventory` self _output_get_2))
    (:`then_2`
      (`self.SetInventoryDimensions`))))

(event `self.HandleItemOnClicked`
  (params (ClickedItem :type "/Game/Gameplay/InventorySystem/ItemInterfaces/IBP_Item Interface"))
  (if (`self.InCombineItemMode`)
    (bind _asibp_combinable (cast `/Game/Gameplay/InventorySystem/ItemInterfaces/IBP_Combinable` (`self.ActiveItem`))
      (:`then`
        (bind _asibp_combinable_2 (cast `/Game/Gameplay/InventorySystem/ItemInterfaces/IBP_Combinable` ClickedItem)
          (:`then`
            ;[1 1 1] Both cast succeed: Both items are combinable.
            (`/Game/Gameplay/InventorySystem/ItemInterfaces/IBP_Combinable.Combine` _asibp_combinable _asibp_combinable_2))
          (:`CastFailed`
            ;[1 1 1] Either cast fail: At least one item isn't combinable.
            (`KismetSystemLibrary.PrintString` "Item is not combinable!" :!label _label))))
      (:`CastFailed`
        (goto _label)))
    ;[1 1 1] Finish combine.
    (`self.ExitItemCombineMode`)
    (`self.HideItemMenu`)
    (else
      (bind _output_get (set `self.ActiveItem` ClickedItem))
      (`self.ShowItemMenu` _output_get))))

(fn `AddItem`
  (params (ItemToAdd :type "/Game/Gameplay/InventorySystem/ItemInterfaces/IBP_Item Interface"))
  (returns (Successful :type Boolean))
  (locals (ItemIndex :type Integer))
  (bind _inventorygridmaxcolumns (`self.InventoryGridMaxColumns`))
  (bind _itemindex (`local.ItemIndex`))
  ;[1 1 1] Is inventory full?
  (bind _itemcount (`self.CountItem`))
  (if (>= _itemcount (`self.InventoryMaxStorage`))
    (`/Game/Gameplay/BPFuncLib_Utilities.DisplayNotification` "Inventory is full!")
    (return false)
    (else
      ;[1 1 1] Add this item, and update its CurrentInventory..
      (bind _returnvalue (`KismetArrayLibrary.Array_Add` (`self.Items`) ItemToAdd))
      (set `local.ItemIndex` _returnvalue)
      (`/Game/Gameplay/InventorySystem/ItemInterfaces/IBP_Item.SetCurrentInventory` ItemToAdd self)
      ;[1 1 1] Add item widget to grid.
      (bind _itemwidget (`/Game/Gameplay/InventorySystem/ItemInterfaces/IBP_Item.GetItemWidget` ItemToAdd))
      (bind _returnvalue_2 (`GridPanel.AddChildToGrid` (`self.GridPanelOfItems`) _itemwidget))
      (`GridSlot.SetColumn` _returnvalue_2 (mod _itemindex _inventorygridmaxcolumns))
      (`GridSlot.SetRow` _returnvalue_2 (/ _itemindex _inventorygridmaxcolumns))
      (return true))))

(fn `CountItem`
  (returns (ItemCount :type Integer))
  (return (`KismetArrayLibrary.Array_Length` (`self.Items`))))

(fn `EnterItemCombineMode`
  (set `self.InCombineItemMode` true))

(fn `ExitItemCombineMode`
  (set `self.InCombineItemMode` false))

(fn `HideInventory`
  (if (`Widget.IsInViewport` (`self.InventoryWidget`))
    (`Widget.RemoveFromParent` (`self.InventoryWidget`))
    (`self.HideItemMenu`)
    (`self.ExitItemCombineMode`)
    (else
      (`KismetSystemLibrary.PrintString` "Something has tried to call BP_InventoryComponent's HideInventory function, when WBP_Inventory is not in viewport!" true true (struct :`R` 1.0 :`G` 1.0 :`A` 1.0) 10.0))))

(fn `HideItemMenu`
  (bind _wbp_itemmenu (`self.WBP_ItemMenu`))
  (if (`Widget.IsInViewport` _wbp_itemmenu)
    (`Widget.RemoveFromParent` _wbp_itemmenu)))

(fn `RemoveItem`
  (params (ItemToRemove :type "/Game/Gameplay/InventorySystem/ItemInterfaces/IBP_Item Interface"))
  (returns (Successful :type Boolean))
  (bind _inventorygridmaxcolumns (`self.InventoryGridMaxColumns`))
  (bind _gridpanelofitems (`self.GridPanelOfItems`))
  (`|ExecutionSequence`
    (:`then_0`
      ;[1 1 1] Backend array removal
      (`KismetArrayLibrary.Array_RemoveItem` (`self.Items`) ItemToRemove))
    (:`then_1`
      ;[1 1 1] Reset ActiveItem to nothing.
      (set `self.ActiveItem` null))
    (:`then_2`
      ;[1 1 1] Clear the grid panel, then re-add, because grid panel's "Remove Child" seems broken.
      (`PanelWidget.ClearChildren` _gridpanelofitems)
      (for (_array_element _array_index) (`self.Items`)
        (bind _itemwidget (`/Game/Gameplay/InventorySystem/ItemInterfaces/IBP_Item.GetItemWidget` _array_element))
        (bind _returnvalue (`GridPanel.AddChildToGrid` _gridpanelofitems _itemwidget))
        (`GridSlot.SetColumn` _returnvalue (mod _array_index _inventorygridmaxcolumns))
        (`GridSlot.SetRow` _returnvalue (/ _array_index _inventorygridmaxcolumns))))
    (:`then_3`
      (return true))))

(fn `SendItem`
  (params (ItemToSend :type "/Game/Gameplay/InventorySystem/ItemInterfaces/IBP_Item Interface"))
  ;[1 1 1] Is the owner BP_User in a waypoint?
  (bind _asbp_user (cast `/Game/Gameplay/BP_User` (`self.GetOwner`)))
  (bind _returnvalue (`E2EECharacter.GetCurrentWaypoint` _asbp_user))
  (if (`KismetSystemLibrary.IsValid` _returnvalue)
    ;[1 1 1] Is there a BP_Messenger in the waypoint?
    (for _array_element (`Waypoint.GetOccupants` _returnvalue)
      (cast `/Game/Gameplay/BP_Messenger` _array_element)
      ;[1 1 1] Send the item.
      (`self.RemoveItem` (`local.ItemToSend`))
      (`/Game/Gameplay/BP_Messenger.StartDeliverItem` (`self.TheMessenger`) (`local.ItemToSend`))
      (return)))
  ;[1 1 1] Conditions aren't met.
  (`/Game/Gameplay/BPFuncLib_Utilities.DisplayNotification` "Get close to the Messenger before sending items.")
  (return))

(fn `SetInventoryDimensions`
  (bind _returnvalue (`|CreateWidget` "/Game/UI/ItemWidgets/WBP_Lock.WBP_Lock_C"))
  (bind (_returnvalue_x _returnvalue_y) (`KismetMathLibrary.BreakVector2D` (/ (`CanvasPanelSlot.GetSize` (`WidgetLayoutLibrary.SlotAsCanvasSlot` (`self.GridPanelOfItems`))) (`.ImageSize` (break `SlateBrush` (`Image.Brush` (`/Game/UI/ItemWidgets/WBP_Lock.Image_Icon` _returnvalue)))))))
  (bind _output_get (set `self.InventoryGridMaxColumns` (`KismetMathLibrary.FTrunc` _returnvalue_x)))
  (bind _output_get_2 (set `self.InventoryGridMaxRows` (`KismetMathLibrary.FTrunc` _returnvalue_y)))
  (set `self.InventoryMaxStorage` (* _output_get_2 _output_get)))

(fn `ShowInventory`
  (if (`Widget.IsInViewport` (`self.InventoryWidget`))
    (`KismetSystemLibrary.PrintString` "Something has tried to call BP_InventoryComponent's ShowInventory function, when WBP_Inventory is already in viewport!" true true (struct :`R` 1.0 :`G` 1.0 :`A` 1.0) 10.0)
    (else
      (`UserWidget.AddToViewport` (`self.InventoryWidget`) 0))))

(fn `ShowItemMenu`
  (params (ActiveItem :type "/Game/Gameplay/InventorySystem/ItemInterfaces/IBP_Item Interface"))
  (bind _wbp_itemmenu (`self.WBP_ItemMenu`))
  (`/Game/UI/WBP_ItemMenu.FormMenu` _wbp_itemmenu ActiveItem)
  (if (not (`Widget.IsInViewport` _wbp_itemmenu))
    (`UserWidget.AddToViewport` _wbp_itemmenu 0))
  (bind _returnvalue (`WidgetLayoutLibrary.GetMousePositionOnViewport`))
  (`UserWidget.SetPositionInViewport` _wbp_itemmenu _returnvalue false))

(fn `ShowNotification`
  (params (NotificationString :type String))
  (bind _asbp_my_player_controller (cast `/Game/Gameplay/BP_MyPlayerController` (`GameplayStatics.GetPlayerController` 0)))
  (`/Game/Gameplay/BP_MyPlayerController.DisplayNotification` _asbp_my_player_controller NotificationString))