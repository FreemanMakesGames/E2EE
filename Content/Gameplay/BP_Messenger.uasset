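; Messenger character that carries items between Alice's and Bob's waypoints, secretly or otherwise retaining keys it handles.
; Clicking it opens a menu widget at the cursor; hovering highlights its mesh.
; StartDeliverItem records keys in its inventory, including those inside locked containers it has matching keys for, and sends its AI controller toward the other waypoint.
; Overlapping a waypoint re-enables the carried item and teleports it to the drop-off point.
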(event `self.ReceiveBeginPlay`
  (bind _returnvalue (`|CreateWidget` "/Game/UI/WBP_MessengerMenu.WBP_MessengerMenu_C" null self))
  (set `self.WBP_MessengerMenu` _returnvalue))

(event `self.CapsuleComponent.OnClicked`
  (params (TouchedComponent :type "PrimitiveComponent Object Reference") (ButtonPressed :type "Key Structure"))
  (bind _wbp_messengermenu (`self.WBP_MessengerMenu`))
  (if (not (`Widget.IsInViewport` _wbp_messengermenu))
    (`UserWidget.AddToViewport` _wbp_messengermenu 0))
  (bind _returnvalue (`WidgetLayoutLibrary.GetMousePositionOnViewport`))
  (`UserWidget.SetPositionInViewport` _wbp_messengermenu _returnvalue false))

(event `self.CapsuleComponent.OnBeginCursorOver`
  (params (TouchedComponent :type "PrimitiveComponent Object Reference"))
  ;[1 1 1] Highlight
  (`HighlightComponent.Highlight` (`self.Highlight`) (`self.Mesh`)))

(event `self.CapsuleComponent.OnEndCursorOver`
  (params (TouchedComponent :type "PrimitiveComponent Object Reference"))
  ;[1 1 1] Highlight
  (`HighlightComponent.EndHighlight` (`self.Highlight`) (`self.Mesh`)))

(event `self.CapsuleComponent.OnComponentBeginOverlap`
  (params (OverlappedComponent :type "PrimitiveComponent Object Reference") (OtherActor :type "Actor Object Reference") (OtherComp :type "PrimitiveComponent Object Reference") (OtherBodyIndex :type Integer) (bFromSweep :type Boolean) (SweepResult :type "HitResult Structure (by ref)"))
  (bind _aswaypoint (cast `Waypoint` OtherActor))
  (`self.OnArrivingWaypoint` _aswaypoint))

(fn `CloneItem`
  (params (ItemToClone :type "/Game/Gameplay/InventorySystem/ItemInterfaces/IBP_Item Interface"))
  (cast `/Game/Props/Blueprints/BP_Message` ItemToClone
    (:`then`)
    (:`CastFailed`
      (bind _asbp_key (cast `/Game/Props/Blueprints/BP_Key` (`local.ItemToClone`))
        (:`then`
          (`/Game/Gameplay/InventorySystem/BP_MessengerInventory.AddItem` (`self.MyInventory`) _asbp_key))
        (:`CastFailed`
          (bind _asbp_container (cast `/Game/Props/Blueprints/BP_Container` (`local.ItemToClone`)))
          (bind _currentlock (`/Game/Props/Blueprints/BP_Container.CurrentLock` _asbp_container))
          (if (`KismetSystemLibrary.IsValid` _currentlock)
            (bind _id (`/Game/Props/Blueprints/BP_Lock.GetID` _currentlock))
            (bind _found (`self.FindKey` _id))
            (if _found
              (bind _containeditem (`/Game/Props/Blueprints/BP_Container.ContainedItem` _asbp_container))
              (cast `/Game/Props/Blueprints/BP_Message` _containeditem
                (:`then`)
                (:`CastFailed`
                  (bind _asbp_key_2 (cast `/Game/Props/Blueprints/BP_Key` _containeditem))
                  (`/Game/Gameplay/InventorySystem/BP_MessengerInventory.AddItem` (`self.MyInventory`) _asbp_key_2))))))))))

(fn `FindKey`
  (params (QueriedID :type Integer))
  (returns (Found :type Boolean))
  (for _array_element (`/Game/Gameplay/InventorySystem/BP_MessengerInventory.Items` (`self.MyInventory`))
    (bind _asbp_key (cast `/Game/Props/Blueprints/BP_Key` _array_element))
    (bind _id (`/Game/Props/Blueprints/BP_Key.GetID` _asbp_key))
    (if (== _id (`local.QueriedID`))
      (return true)))
  (return false))

(fn `HideMessengerMenu`
  (bind _wbp_messengermenu (`self.WBP_MessengerMenu`))
  (if (`Widget.IsInViewport` _wbp_messengermenu)
    (`Widget.RemoveFromParent` _wbp_messengermenu)))

(fn `OnArrivingWaypoint`
  (params (TheWaypoint :type "Waypoint Object Reference"))
  (if (`KismetSystemLibrary.IsValid` (`KismetSystemLibrary.Conv_InterfaceToObject` (`self.CarryingItem`)))
    ;[1 1 1] Re-enable item actor, and move it to drop off point.
    (bind _asactor (cast `Actor` (`KismetSystemLibrary.Conv_InterfaceToObject` (`self.CarryingItem`))))
    (`/Game/Gameplay/BPFuncLib_Utilities.CompletelyEnableActorWithPrimitiveComponent` _asactor)
    (`self.K2_SetActorLocation` _asactor (`Waypoint.GetDefaultItemDropOffLocation` (`local.TheWaypoint`)) false true)
    (set `self.CarryingItem` null)))

(fn `StartDeliverItem`
  (params (ItemToDeliver :type "/Game/Gameplay/InventorySystem/ItemInterfaces/IBP_Item Interface"))
  (locals (TargetWaypoint :type "Waypoint Object Reference"))
  (set `self.CarryingItem` ItemToDeliver)
  (`AIController.MoveToActor` (`self.MyAIController`) (`self.MiddlePoint`) -1.0 true true true null true)
  (`self.CloneItem` (`self.CarryingItem`))
  ;[1 1 1] Move to target waypoint.
  (bind _returnvalue (`self.GetCurrentWayPoint`))
  (if (== _returnvalue (`self.Waypoint_Alice`))
    (set `local.TargetWaypoint` (`self.Waypoint_Bob`))
    (else
      (set `local.TargetWaypoint` (`self.Waypoint_Alice`))))
  (`AIController.MoveToActor` (`self.MyAIController`) (`local.TargetWaypoint`) -1.0 true true true null true))

(fn `UserConstructionScript`)