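; Obsolete lock item actor that carries a LockID, going by its name a superseded version of the lock.
; SetID stores the ID and writes it with a "#" prefix to the WBP_Lock item widget's text, while GetID returns it.
; Duplicate spawns another lock of the same class, copies the ID onto it, disables it and returns it.
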(fn `Duplicate`
  (returns (ReturnValue :type "Item Object Reference"))
  (bind _returnvalue (`|SpawnActorFromClass` "Obsolete_BP_Lock_C" (`KismetMathLibrary.MakeTransform` (0.0 0.0 0.0)) "Undefined" "OverrideRootScale" null null))
  (`self.SetID` _returnvalue (`self.LockID`))
  (`GameUtilities.DisableActor` _returnvalue)
  (return _returnvalue))

(fn `GetID`
  (returns (ID :type Integer))
  (return (`self.LockID`)))

(fn `SetID`
  (params (ID :type Integer))
  (set `self.LockID` ID)
  (bind _aswbp_lock (cast `/Game/UI/InventorySystem/ItemWidgets/WBP_Lock` (`self.ItemWidget`)))
  (`TextBlock.SetText` (`/Game/UI/InventorySystem/ItemWidgets/WBP_Lock.TextBlock_ID` _aswbp_lock) (`KismetTextLibrary.Conv_StringToText` (`KismetStringLibrary.Concat_StrStr` "#" (`KismetStringLibrary.Conv_IntToString` (`self.LockID`))))))

(fn `UserConstructionScript`)