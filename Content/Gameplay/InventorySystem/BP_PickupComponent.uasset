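; BP_PickupComponent is an actor component that lets the player pick up its owning Item by clicking it.
; On BeginPlay it binds OnClicked on the owner's primitive component, or prints an error if the owner is not an Item.
; Pickup checks that the controller's ActiveCharacter is within PickupRange, then adds the Item to that character's Inventory.
; The picked-up actor is disabled rather than destroyed, retaining its data.
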(event `self.ReceiveBeginPlay`
  ;[1 1 1] Check and set IBP_Item.
  (bind _asitem (cast `Item` (`self.GetOwner`))
    (:`then`
      (set `self.OwnerItem` _asitem)
      ;[1 1 1] Bind OnClicked.
      (add `PrimitiveComponent.OnClicked` (`Actor.GetComponentByClass` (`self.GetOwner`) "/Script/Engine.PrimitiveComponent") (delegate `OnClicked`)))
    (:`CastFailed`
      (`KismetSystemLibrary.PrintString` "BP_PickupComponent is added to a non-Item!" true true (struct :`R` 1.0 :`A` 1.0) 100.0))))

(event `OnClicked`
  (params (TouchedComponent :type "PrimitiveComponent Object Reference") (ButtonPressed :type "Key Structure"))
  ;[1 1 1] Bind OnClicked.
  (`self.Pickup`))

(fn `Pickup`
  (locals (ActiveCharacter :type "E2EECharacter Object Reference") (ActiveInventory :type "Inventory Object Reference"))
  (`|ExecutionSequence`
    (:`then_0`
      ;[1 1 1] Get and check ActiveCharacter.
      (bind _asbp_my_player_controller (cast `/Game/Gameplay/BP_MyPlayerController` (`GameplayStatics.GetPlayerController` 0)))
      (bind _output_get (set `local.ActiveCharacter` (`MyPlayerController.ActiveCharacter` _asbp_my_player_controller)))
      (if (not (`KismetSystemLibrary.IsValid` _output_get))
        (return)))
    (:`then_1`
      ;[1 1 1] Check if ActiveCharacter is within PickupRange.
      (if (not (<= (`KismetMathLibrary.VSize` (- (`Actor.K2_GetActorLocation` (`self.GetOwner`)) (`Actor.K2_GetActorLocation` (`local.ActiveCharacter`)))) (`self.PickupRange`)))
        (`/Game/Gameplay/BPFuncLib_Utilities.DisplayNotification` "Too far to pick up this item")
        (return)))
    (:`then_2`
      ;[1 1 1] Set ActiveInventory.
      (set `local.ActiveInventory` (`Actor.GetComponentByClass` (`local.ActiveCharacter`) "/Script/E2EE.Inventory")))
    (:`then_3`
      ;[1 1 1] Set and add to current inventory.
      (`Inventory.AddItem` (`local.ActiveInventory`) (`self.OwnerItem`))
      (if true
        ;[1 1 1] Disable owner in game, but retain its data.
        (`/Game/Gameplay/BPFuncLib_Utilities.CompletelyDisableActorWithPrimitiveComponent` (`self.GetOwner`))))))