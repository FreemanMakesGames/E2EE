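; Basic player controller that manages the player's notification widget and inventory menu.
; On BeginPlay it creates a notification widget and adds it to the viewport, then forwards DisplayNotification event text to it.
; The Tab key toggles the inventory, hiding the menu when it is in the viewport and otherwise calling ShowInventoryMenu.
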(event `self.ReceiveBeginPlay`
  (bind _returnvalue (`|CreateWidget` "/Game/UI/WBP_Notification.WBP_Notification_C"))
  (bind _output_get (set `self.WBP_Notification` _returnvalue))
  (`UserWidget.AddToViewport` _output_get 0))

(event `Key|Tab`
  (params (Key :type "Key Structure"))
  (:`Pressed`
    (if (`Widget.IsInViewport` (`self.InventoryMenu`))
      (`InventoryMenu.HideInventory` (`self.InventoryMenu`))
      (else
        (`self.ShowInventoryMenu`)))))

(event `self.DisplayNotification`
  (params (NotificationText :type "Text (by ref)"))
  (`Notification.DisplayNotification` (`self.WBP_Notification`) NotificationText))

(fn `UserConstructionScript`)