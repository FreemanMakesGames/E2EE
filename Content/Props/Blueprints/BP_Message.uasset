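; BP_Message is an inventory item prop representing a message that can be combined with containers.
; On BeginPlay it creates its own Obsolete_WBP_Message widget, and clicks on that item are forwarded to the current inventory.
; Combine delegates to an Obsolete_BP_Container target and shows a notification for any other target.
; Getters expose its name, icon, widget, inventory and "Combine" usage label, and Destroy removes the actor.
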(event `self.ReceiveBeginPlay`
  (bind _returnvalue (`|CreateWidget` "/Game/UI/ItemWidgets/Obsolete_WBP_Message.Obsolete_WBP_Message_C" null self))
  (set `self.ItemWidget` _returnvalue))

(event `/Game/Gameplay/InventorySystem/ItemInterfaces/IBP_Item.SetCurrentInventory`
  (params (CurrentInventory :type "/Game/Gameplay/InventorySystem/BP_InventoryComponent Object Reference"))
  (set `self.CurrentInventory` CurrentInventory))

(event `/Game/Gameplay/InventorySystem/ItemInterfaces/IBP_Combinable.Combine`
  (params (TargetItem :type "/Game/Gameplay/InventorySystem/ItemInterfaces/IBP_Combinable Interface"))
  (bind _asobsolete_bp_container (cast `/Game/Props/Blueprints/Obsolete_BP_Container` TargetItem)
    (:`then`
      (`/Game/Props/Blueprints/Obsolete_BP_Container.Combine` _asobsolete_bp_container self))
    (:`CastFailed`
      (`/Game/Gameplay/BPFuncLib_Utilities.DisplayNotification` "Message can only be combined with a container."))))

(event `/Game/Gameplay/InventorySystem/ItemInterfaces/IBP_Destroyable.Destroy`
  (`self.K2_DestroyActor`))

(fn `GetCombineUsageName`
  (returns (CombineUsageName :type String))
  (return "Combine"))

(fn `GetCurrentInventory`
  (returns (CurrentInventory :type "/Game/Gameplay/InventorySystem/BP_InventoryComponent Object Reference"))
  (return (`self.CurrentInventory`)))

(fn `GetItemIcon`
  (returns (ItemIcon :type "Texture2D Object Reference"))
  (return (`self.ItemIcon`)))

(fn `GetItemName`
  (returns (ItemName :type String))
  (return (`self.ItemName`)))

(fn `GetItemWidget`
  (returns (ItemWidget :type "UserWidget Object Reference"))
  (return (`self.ItemWidget`)))

(fn `HandleItemWidgetOnClicked`
  (`/Game/Gameplay/InventorySystem/BP_InventoryComponent.HandleItemOnClicked` (`self.CurrentInventory`) self))

(fn `UserConstructionScript`)