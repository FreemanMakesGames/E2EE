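; Obsolete lock prop that acts as an inventory item and can be combined with keys or containers.
; On BeginPlay it creates its own item widget, whose clicks are forwarded to the current inventory.
; Combine casts the target: keys only trigger a match or mismatch notification by ID, containers get locked with this lock, and other targets are rejected.
; Getters expose item data, and cursor hover highlights the mesh.
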(event `self.ReceiveBeginPlay`
  (bind _returnvalue (`|CreateWidget` "/Game/UI/ItemWidgets/Obsolete_WBP_Lock.Obsolete_WBP_Lock_C"))
  (bind _output_get (set `self.ItemWidget` _returnvalue))
  (`/Game/UI/ItemWidgets/Obsolete_WBP_Lock.Initialize` _output_get self))

(event `/Game/Gameplay/InventorySystem/ItemInterfaces/IBP_Item.SetCurrentInventory`
  (params (CurrentInventory :type "/Game/Gameplay/InventorySystem/BP_InventoryComponent Object Reference"))
  (set `self.CurrentInventory` CurrentInventory))

(event `/Game/Gameplay/InventorySystem/ItemInterfaces/IBP_Combinable.Combine`
  (params (TargetItem :type "/Game/Gameplay/InventorySystem/ItemInterfaces/IBP_Combinable Interface"))
  (if (== (`KismetSystemLibrary.Conv_InterfaceToObject` TargetItem) self)
    ;[1 1 1] Combining with myself
    (`/Game/Gameplay/BPFuncLib_Utilities.DisplayNotification` "A lock can't lock itself.")
    (else
      (bind _asobsolete_bp_key (cast `/Game/Props/Blueprints/Obsolete_BP_Key` TargetItem)
        (:`then`
          ;[1 1 1] Combining with a key
          (if (== (`/Game/Props/Blueprints/Obsolete_BP_Key.KeyID` _asobsolete_bp_key) (`self.LockID`))
            (`/Game/Gameplay/BPFuncLib_Utilities.DisplayNotification` "Lock and key match!")
            (else
              (`/Game/Gameplay/BPFuncLib_Utilities.DisplayNotification` "Lock and key don't match!"))))
        (:`CastFailed`
          ;[1 1 1] Combining with a container
          (bind _asbp_container (cast `/Game/Props/Blueprints/BP_Container` TargetItem)
            (:`then`
              (`/Game/Props/Blueprints/BP_Container.Lock` _asbp_container self))
            (:`CastFailed`
              (`/Game/Gameplay/BPFuncLib_Utilities.DisplayNotification` "Lock can't be combined with this item."))))))))

(event `/Game/Gameplay/InventorySystem/ItemInterfaces/IBP_Destroyable.Destroy`
  (`self.K2_DestroyActor`))

(event `self.StaticMesh.OnBeginCursorOver`
  (params (TouchedComponent :type "PrimitiveComponent Object Reference"))
  ;[1 1 1] Highlight
  (`HighlightComponent.Highlight` (`self.Highlight`) (`self.StaticMesh`)))

(event `self.StaticMesh.OnEndCursorOver`
  (params (TouchedComponent :type "PrimitiveComponent Object Reference"))
  ;[1 1 1] Highlight
  (`HighlightComponent.EndHighlight` (`self.Highlight`) (`self.StaticMesh`)))

(fn `GetCombineUsageName`
  (returns (CombineUsageName :type String))
  (return "Lock"))

(fn `GetCurrentInventory`
  (returns (CurrentInventory :type "/Game/Gameplay/InventorySystem/BP_InventoryComponent Object Reference"))
  (return (`self.CurrentInventory`)))

(fn `GetID`
  (returns (ID :type Integer))
  (return (`self.LockID`)))

(fn `GetItemIcon`
  (returns (ItemIcon :type "Texture2D Object Reference"))
  (return (`self.ItemIcon`)))

(fn `GetItemName`
  (returns (ItemName :type String))
  (return (`self.ItemName`)))

(fn `GetItemWidget`
  (returns (ItemWidget :type "UserWidget Object Reference"))
  (return (`self.ItemWidget`)))

(fn `HandleItemWidgetOnClicked`
  (`/Game/Gameplay/InventorySystem/BP_InventoryComponent.HandleItemOnClicked` (`self.CurrentInventory`) self))

(fn `UserConstructionScript`
  (`parent.UserConstructionScript`))