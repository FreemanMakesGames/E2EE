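; Player controller for the home menu, with the mouse cursor and click and hover events enabled.
; On BeginPlay it creates the home and option menu widgets and shows the home menu.
; DisplayOptionMenu adds the option menu to the viewport and pushes it onto a menu stack.
; Q or Escape pops and removes the topmost stacked menu, while the home menu stays outside the stack.
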(event `self.ReceiveBeginPlay`
  (`|ExecutionSequence`
    (:`then_0`
      (set `self.bShowMouseCursor` true)
      (set `self.bEnableClickEvents` true)
      (set `self.bEnableMouseOverEvents` true))
    (:`then_1`
      (bind _returnvalue (`|CreateWidget` "/Game/UI/Menus/WBP_HomeMenu.WBP_HomeMenu_C" null self))
      (set `self.HomeMenu` _returnvalue)
      (bind _returnvalue_2 (`|CreateWidget` "/Game/UI/Menus/WBP_OptionMenu.WBP_OptionMenu_C" null self))
      (set `self.OptionMenu` _returnvalue_2))
    (:`then_2`
      (`self.DisplayHomeMenu`))))

(event `Key|Q`
  (params (Key :type "Key Structure"))
  (:`Pressed`
    (`self.RemoveTopMostMenu` :!label _label)))

(event `Key|Escape`
  (params (Key :type "Key Structure"))
  (:`Pressed`
    (goto _label)))

(fn `DisplayHomeMenu`
  (`UserWidget.AddToViewport` (`self.HomeMenu`) 0))

(fn `DisplayOptionMenu`
  (bind _optionmenu (`self.OptionMenu`))
  (`UserWidget.AddToViewport` _optionmenu 0)
  (`KismetArrayLibrary.Array_Add` (`self.DisplayedMenuStack`) _optionmenu))

(fn `RemoveTopMostMenu`
  (bind _displayedmenustack (`self.DisplayedMenuStack`))
  (bind _returnvalue (`KismetArrayLibrary.Array_LastIndex` _displayedmenustack))
  (if (> (`KismetArrayLibrary.Array_Length` (`self.DisplayedMenuStack`)) 0)
    (`Widget.RemoveFromParent` (`|GetArrayItem` _displayedmenustack _returnvalue))
    (`KismetArrayLibrary.Array_Remove` _displayedmenustack _returnvalue)))

(fn `UserConstructionScript`)