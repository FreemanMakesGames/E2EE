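; BP_Inventory handles open and read actions on inventory items for its owning actor.
; Opening a container item checks its lock and occupancy, then either moves the released item into the inventory or shows a locked or empty notification.
; Reading is forwarded to the owning BP_BasicCharacter, with a notification and warning when the owner is not that character type.
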(event `self.OpenItem`
  (params (ItemToOpen :type "ItemInfo Object Reference"))
  (bind _ascontainer_item_info (cast `ContainerItemInfo` ItemToOpen))
  (bind _returnvalue (`ContainerItemInfo.IsLocked` _ascontainer_item_info))
  (if _returnvalue
    (`/Game/Gameplay/BPFuncLib_Utilities.DisplayNotification` "This container is locked!")
    (else
      (bind _returnvalue_2 (`ContainerItemInfo.IsOccupied` _ascontainer_item_info))
      (if _returnvalue_2
        (bind _returnvalue_3 (`ContainerItemInfo.ReleaseItem` _ascontainer_item_info))
        (`self.AddItem` _returnvalue_3)
        (else
          (`/Game/Gameplay/BPFuncLib_Utilities.DisplayNotification` "This container is empty!"))))))

(event `self.ReadItem`
  (params (ItemToRead :type "ItemInfo Object Reference"))
  (bind _asbp_basic_character (cast `/Game/Characters/BP_BasicCharacter` (`self.GetOwner`))
    (:`then`
      (`/Game/Characters/BP_BasicCharacter.ReadItem` _asbp_basic_character ItemToRead))
    (:`CastFailed`
      (`/Game/Gameplay/BPFuncLib_Utilities.DisplayNotification` "Only Users can read Messages!")
      (`DevUtilities.PrintWarning` "Are you controlling a non-User Actor?"))))