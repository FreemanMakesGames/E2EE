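; Inventory item container that holds one other item and can be secured with a lock.
; Combine moves a non-container item from the current inventory inside, and Use returns it unless locked.
; Lock consumes a lock item; Unlock compares key and lock IDs, destroying the lock and consuming the key on a match.
; Its UMG widget icon reflects open, closed or locked state, and the mesh highlights on cursor hover.
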(event `self.ReceiveBeginPlay`
  (bind _returnvalue (`|CreateWidget` "/Game/UI/ItemWidgets/WBP_Container.WBP_Container_C"))
  (bind _output_get (set `self.ItemWidget` _returnvalue))
  (`/Game/UI/ItemWidgets/WBP_Container.Initialize` _output_get self))

(event `/Game/Gameplay/InventorySystem/ItemInterfaces/IBP_Item.SetCurrentInventory`
  (params (CurrentInventory :type "/Game/Gameplay/InventorySystem/BP_InventoryComponent Object Reference"))
  (set `self.CurrentInventory` CurrentInventory))

(event `/Game/Gameplay/InventorySystem/ItemInterfaces/IBP_Usable.Use`
  ;[1 1 1] Locked?
  (bind _islocked (`self.IsLocked`))
  (if _islocked
    (`/Game/Gameplay/BPFuncLib_Utilities.DisplayNotification` (`KismetStringLibrary.Concat_StrStr` "This container is locked by lock #" (`KismetStringLibrary.Conv_IntToString` (`/Game/Props/Blueprints/BP_Lock.LockID` (`self.CurrentLock`)))))
    (else
      ;[1 1 1] Occupied?
      (bind _isoccupied (`self.IsOccupied`))
      (if _isoccupied
        ;[1 1 1] Release ContainedItem to CurrentInventory.
        (bind _additionsuccess (`/Game/Gameplay/InventorySystem/BP_InventoryComponent.AddItem` (`self.CurrentInventory`) (`self.ContainedItem`)))
        (if _additionsuccess
          ;[1 1 1] Reset ContainedItem.
          (set `self.ContainedItem` null)
          ;[1 1 1] Set item widget image.
          (`Image.SetBrushFromTexture` (`/Game/UI/ItemWidgets/WBP_Container.Image_Icon` (`self.ItemWidget`)) "/Game/Props/Icons/ContainerIcon_Opened.ContainerIcon_Opened" false))
        (else
          (`/Game/Gameplay/BPFuncLib_Utilities.DisplayNotification` "This container is empty!"))))))

(event `/Game/Gameplay/InventorySystem/ItemInterfaces/IBP_Combinable.Combine`
  (params (TargetItem :type "/Game/Gameplay/InventorySystem/ItemInterfaces/IBP_Combinable Interface"))
  (bind _returnvalue (`KismetSystemLibrary.Conv_InterfaceToObject` TargetItem))
  ;[1 1 1] Combining with self?
  (if (== (`KismetSystemLibrary.Conv_InterfaceToObject` TargetItem) self)
    (`/Game/Gameplay/BPFuncLib_Utilities.DisplayNotification` "A container can't contain itself.")
    (else
      (bind _islocked (`self.IsLocked`))
      (if _islocked
        (`/Game/Gameplay/BPFuncLib_Utilities.DisplayNotification` "This container is locked!")
        (else
          (bind _isoccupied (`self.IsOccupied`))
          (if _isoccupied
            (`/Game/Gameplay/BPFuncLib_Utilities.DisplayNotification` "This container is already occupied!")
            (else
              ;[1 1 1] Is it another container?
              (if (== (`GameplayStatics.GetObjectClass` _returnvalue) "BP_Container_C")
                (`/Game/Gameplay/BPFuncLib_Utilities.DisplayNotification` "Naughty! We've disabled putting a container into another container...")
                (else
                  ;[1 1 1] Contain TargetItem.
                  (bind _asibp_item (cast `/Game/Gameplay/InventorySystem/ItemInterfaces/IBP_Item` _returnvalue))
                  (set `self.ContainedItem` _asibp_item)
                  ;[1 1 1] Remove TargetItem from CurrentInventory.
                  (`/Game/Gameplay/InventorySystem/BP_InventoryComponent.RemoveItem` (`self.CurrentInventory`) _asibp_item)
                  ;[1 1 1] Change my icon.
                  (`Image.SetBrushFromTexture` (`/Game/UI/ItemWidgets/WBP_Container.Image_Icon` (`self.ItemWidget`)) "/Game/Props/Icons/ContainerIcon_Closed.ContainerIcon_Closed" false))))))))))

(event `/Game/Gameplay/InventorySystem/ItemInterfaces/IBP_Destroyable.Destroy`
  (`self.K2_DestroyActor`))

(event `self.StaticMesh.OnBeginCursorOver`
  (params (TouchedComponent :type "PrimitiveComponent Object Reference"))
  ;[1 1 1] Highlight
  (`HighlightComponent.Highlight` (`self.Highlight`) (`self.StaticMesh`)))

(event `self.StaticMesh.OnEndCursorOver`
  (params (TouchedComponent :type "PrimitiveComponent Object Reference"))
  ;[1 1 1] Highlight
  (`HighlightComponent.EndHighlight` (`self.Highlight`) (`self.StaticMesh`)))

(fn `GetCombineUsageName`
  (returns (CombineUsageName :type String))
  (return "Contain"))

(fn `GetCurrentInventory`
  (returns (CurrentInventory :type "/Game/Gameplay/InventorySystem/BP_InventoryComponent Object Reference"))
  (return (`self.CurrentInventory`)))

(fn `GetItemIcon`
  (returns (ItemIcon :type "Texture2D Object Reference"))
  (return (`self.ItemIcon`)))

(fn `GetItemName`
  (returns (ItemName :type String))
  (return (`self.ItemName`)))

(fn `GetItemWidget`
  (returns (ItemWidget :type "UserWidget Object Reference"))
  (return (`self.ItemWidget`)))

(fn `GetUsageName`
  (returns (UsageName :type String))
  (return "Open"))

(fn `HandleItemWidgetOnClicked`
  (`/Game/Gameplay/InventorySystem/BP_InventoryComponent.HandleItemOnClicked` (`self.CurrentInventory`) self))

(fn `IsLocked`
  (returns (IsLocked :type Boolean))
  (return (`KismetSystemLibrary.IsValid` (`self.CurrentLock`))))

(fn `IsOccupied`
  (returns (IsOccupied :type Boolean))
  (return (`KismetSystemLibrary.IsValid` (`KismetSystemLibrary.Conv_InterfaceToObject` (`self.ContainedItem`)))))

(fn `Lock`
  (params (NewLock :type "/Game/Props/Blueprints/BP_Lock Object Reference"))
  (bind _newlock (`local.NewLock`))
  ;[1 1 1] Already locked?
  (if (`KismetSystemLibrary.IsValid` (`self.CurrentLock`))
    (`/Game/Gameplay/BPFuncLib_Utilities.DisplayNotification` "This container is already locked!")
    (else
      ;[1 1 1] Lock.
      (set `self.CurrentLock` _newlock)
      ;[1 1 1] Remove the lock from inventory.
      (bind _asibp_item (cast `/Game/Gameplay/InventorySystem/ItemInterfaces/IBP_Item` _newlock))
      (`/Game/Gameplay/InventorySystem/BP_InventoryComponent.RemoveItem` (`self.CurrentInventory`) _asibp_item)
      ;[1 1 1] Set item widget image.
      (`Image.SetBrushFromTexture` (`/Game/UI/ItemWidgets/WBP_Container.Image_Icon` (`self.ItemWidget`)) "/Game/Props/Icons/ContainerIcon_Locked.ContainerIcon_Locked" false))))

(fn `Unlock`
  (params (TheKey :type "/Game/Props/Blueprints/BP_Key Object Reference"))
  (bind _image_icon (`/Game/UI/ItemWidgets/WBP_Container.Image_Icon` (`self.ItemWidget`)))
  ;[1 1 1] Already unlocked?
  (bind _islocked (`self.IsLocked`))
  (if _islocked
    ;[1 1 1] Compare ID.
    (`|ExecutionSequence`
      (:`then_0`
        (bind _id (`/Game/Props/Blueprints/BP_Lock.GetID` (`self.CurrentLock`))))
      (:`then_1`
        (bind _id_2 (`/Game/Props/Blueprints/BP_Key.GetID` (`local.TheKey`))))
      (:`then_2`
        (if (== _id _id_2)
          ;[1 1 1] Unlock.
          (`self.K2_DestroyActor` (`self.CurrentLock`))
          ;[1 1 1] Remove the key from inventory.
          (`/Game/Gameplay/InventorySystem/BP_InventoryComponent.RemoveItem` (`self.CurrentInventory`) (`local.TheKey`))
          ;[1 1 1] Set item widget image.
          (bind _isoccupied (`self.IsOccupied`))
          (if _isoccupied
            (`Image.SetBrushFromTexture` _image_icon "/Game/Props/Icons/ContainerIcon_Closed.ContainerIcon_Closed" false)
            (else
              (`Image.SetBrushFromTexture` _image_icon "/Game/Props/Icons/ContainerIcon_Opened.ContainerIcon_Opened" false)))
          (`/Game/Gameplay/BPFuncLib_Utilities.DisplayNotification` "You unlocked this container.")
          (else
            (`/Game/Gameplay/BPFuncLib_Utilities.DisplayNotification` "The key doesn't match the lock!")))))
    (else
      (`/Game/Gameplay/BPFuncLib_Utilities.DisplayNotification` "This container isn't locked!"))))

(fn `UserConstructionScript`
  (`parent.UserConstructionScript`)
  (bind _asibp_item (cast `/Game/Gameplay/InventorySystem/ItemInterfaces/IBP_Item` self))
  (set `self.MyselfAsIBP_Item` _asibp_item))