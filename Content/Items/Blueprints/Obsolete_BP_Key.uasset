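; Obsolete key item actor that stores a key ID and shows it on its item widget.
; SetID saves the ID and writes it with a "#" prefix into the WBP_Key text block, while GetID returns it.
; Duplicate spawns another key, copies the ID onto it, disables that actor and returns it.
; The event graph and construction script contain no active logic.
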(fn `Duplicate`
  (returns (ReturnValue :type "Item Object Reference"))
  (bind _returnvalue (`|SpawnActorFromClass` "Obsolete_BP_Key_C" (`KismetMathLibrary.MakeTransform` (0.0 0.0 0.0)) "Undefined" "OverrideRootScale" null null))
  (`self.SetID` _returnvalue (`self.KeyID`))
  (`GameUtilities.DisableActor` _returnvalue)
  (return _returnvalue))

(fn `GetID`
  (returns (ID :type Integer))
  (return (`self.KeyID`)))

(fn `SetID`
  (params (ID :type Integer))
  (set `self.KeyID` ID)
  (bind _aswbp_key (cast `/Game/UI/InventorySystem/ItemWidgets/WBP_Key` (`self.ItemWidget`)))
  (`TextBlock.SetText` (`/Game/UI/InventorySystem/ItemWidgets/WBP_Key.TextBlock_ID` _aswbp_key) (`KismetTextLibrary.Conv_StringToText` (`KismetStringLibrary.Concat_StrStr` "#" (`KismetStringLibrary.Conv_IntToString` (`self.KeyID`))))))

(fn `UserConstructionScript`)