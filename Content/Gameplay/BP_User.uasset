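; BP_User is a clickable user actor that opens a context menu widget at the mouse position.
; It creates WBP_UserMenu on BeginPlay with a reference to itself, and HideUserMenu removes it from the viewport.
; Clicking the capsule shows the menu on authority only if IsMessenger, on remote only if not.
; Cursor hover drives mesh highlighting through Highlight, while ToggleWidget sets the visibility of WidgetSelected.
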(event `self.ReceiveBeginPlay`
  (bind _returnvalue (`|CreateWidget` "/Game/UI/WBP_UserMenu.WBP_UserMenu_C" null self))
  (set `self.WBP_UserMenu` _returnvalue))

(event `self.CapsuleComponent.OnClicked`
  (params (TouchedComponent :type "PrimitiveComponent Object Reference") (ButtonPressed :type "Key Structure"))
  (bind _wbp_usermenu (`self.WBP_UserMenu`))
  (`/Engine/EditorBlueprintResources/ActorMacros.Switch Has Authority`
    (:`Authority`
      (if (`self.bIsMessenger`)
        (if (not (`Widget.IsInViewport` _wbp_usermenu)) :!label _label
          (`UserWidget.AddToViewport` _wbp_usermenu 0))
        (bind _returnvalue (`WidgetLayoutLibrary.GetMousePositionOnViewport`))
        (`UserWidget.SetPositionInViewport` _wbp_usermenu _returnvalue false)))
    (:`Remote`
      (if (not (`self.bIsMessenger`))
        (goto _label)))))

(event `self.CapsuleComponent.OnBeginCursorOver`
  (params (TouchedComponent :type "PrimitiveComponent Object Reference"))
  ;[1 1 1] Highlight
  (`HighlightComponent.Highlight` (`self.Highlight`) (`self.Mesh`)))

(event `self.CapsuleComponent.OnEndCursorOver`
  (params (TouchedComponent :type "PrimitiveComponent Object Reference"))
  ;[1 1 1] Highlight
  (`HighlightComponent.EndHighlight` (`self.Highlight`) (`self.Mesh`)))

(event `self.ToggleWidget`
  (params (On :type Boolean))
  (`SceneComponent.SetVisibility` (`self.Widget_Selected`) On false))

(fn `HideUserMenu`
  (bind _wbp_usermenu (`self.WBP_UserMenu`))
  (if (`Widget.IsInViewport` _wbp_usermenu)
    (`Widget.RemoveFromParent` _wbp_usermenu)))

(fn `UserConstructionScript`)