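; Actor component that turns its owning actor into a click-to-pick-up inventory item.
; On BeginPlay it binds to the click event of one of the owner's primitive components.
; A click constructs item data from the configured name and icon, then targets the inventory component on the player controller's active character.
; With free space it adds the item and destroys the owner; otherwise it prints a warning.
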(event `self.ReceiveBeginPlay`
  (add `PrimitiveComponent.OnClicked` (`Actor.GetComponentByClass` (`self.GetOwner`) "/Script/Engine.PrimitiveComponent") (delegate `OnClicked`)))

(event `OnClicked`
  (params (TouchedComponent :type "PrimitiveComponent Object Reference") (ButtonPressed :type "Key Structure"))
  (`self.Pickup`))

(fn `Pickup`
  (locals (ActiveCharacter :type "E2EECharacter Object Reference") (PlayerController :type "/Game/Gameplay/BP_MyPlayerController Object Reference") (BP_InventoryComponent :type "/Game/Gameplay/BP_InventoryComponent Object Reference") (MyItem :type "/Game/Gameplay/BP_InventoryItemData Object Reference"))
  (bind _bp_inventorycomponent (`local.BP_InventoryComponent`))
  (`|ExecutionSequence`
    (:`then_0`
      ;[1 1 1] Setup.
      (bind _asbp_my_player_controller (cast `/Game/Gameplay/BP_MyPlayerController` (`GameplayStatics.GetPlayerController` 0)))
      (bind _output_get (set `local.PlayerController` _asbp_my_player_controller))
      (set `local.ActiveCharacter` (`MyPlayerController.ActiveCharacter` _output_get)))
    (:`then_1`
      ;[1 1 1] Check active character.
      (if (`KismetSystemLibrary.IsValid` (`local.ActiveCharacter`))
        (set `local.BP_InventoryComponent` (`Actor.GetComponentByClass` (`local.ActiveCharacter`) "/Game/Gameplay/BP_InventoryComponent.BP_InventoryComponent_C"))
        (else
          (return))))
    (:`then_2`
      ;[1 1 1] Make MyItem.
      (bind _returnvalue (`|GenericCreateObject` "/Game/Gameplay/BP_InventoryItemData.BP_InventoryItemData_C" self))
      (bind _output_get_2 (set `local.MyItem` _returnvalue))
      (set `/Game/Gameplay/BP_InventoryItemData.Name` (`self.MyItemName`) _output_get_2)
      (set `/Game/Gameplay/BP_InventoryItemData.Icon` (`self.MyItemIcon`) _output_get_2))
    (:`then_3`
      (bind _numberofitems (`/Game/Gameplay/BP_InventoryComponent.CountItems` _bp_inventorycomponent))
      (if (< _numberofitems (`/Game/Gameplay/BP_InventoryComponent.InventoryMaxStorage` _bp_inventorycomponent))
        (`/Game/Gameplay/BP_InventoryComponent.AddItem` (`local.BP_InventoryComponent`) (`local.MyItem`))
        (`Actor.K2_DestroyActor` (`self.GetOwner`))
        (else
          (`KismetSystemLibrary.PrintString` "Too many items" true true (struct :`R` 0.992 :`G` 1.0 :`A` 1.0)))))))