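; BP_MessengerInventory is an inventory that creates WBP_MessengerInventory on BeginPlay and can show or hide it.
; AddItem1 and RemoveItem1 update the item array and grid (removal rebuilds it), with columns and rows derived from panel and lock-icon size.
; SendItem looks for a BP_Messenger at the owning BP_User's waypoint to start delivery, else notifies.
; AddItem, CountItem and RemoveItem, which SendItem calls, are stubs.
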(event `self.ReceiveBeginPlay`
  (`|ExecutionSequence`
    (:`then_0`
      ;[1 1 1] Initialize InventoryWidget.
      (bind _returnvalue (`|CreateWidget` "/Game/UI/WBP_MessengerInventory.WBP_MessengerInventory_C" null self))
      (bind _output_get (set `self.InventoryWidget` _returnvalue))
      ;[1 1 1] Set GridPanelOfItems.
      (set `self.GridPanelOfItems` (`/Game/UI/WBP_MessengerInventory.GridPanel_Items` _output_get)))
    (:`then_2`
      (`self.SetInventoryDimensions`))))

(event `/Game/Gameplay/InventorySystem/IBP_Inventory.HandleItemOnClicked`
  (params (ClickedItem :type "/Game/Gameplay/InventorySystem/ItemInterfaces/IBP_Item Interface")))

(fn `AddItem`
  (params (ItemToAdd :type "/Game/Gameplay/InventorySystem/ItemInterfaces/IBP_Item Interface"))
  (returns (Successful :type Boolean))
  (return false))

(fn `AddItem1`
  (params (NewItem :type "/Game/Gameplay/InventorySystem/ItemInterfaces/IBP_Item Interface"))
  (locals (WBP_Item :type "/Game/UI/WBP_Item Object Reference") (ItemIndex :type Integer :default 0) (NewItemAsActor :type "Actor Object Reference") (NewItemAsObject :type "Object Object Reference"))
  (bind _inventorygridmaxcolumns (`self.InventoryGridMaxColumns`))
  (bind _newitem (`local.NewItem`))
  (bind _itemindex (`local.ItemIndex`))
  ;[1 1 1] Add this item, and set its CurrentInventory.
  (bind _returnvalue (`KismetArrayLibrary.Array_Add` (`self.Items`) _newitem))
  (set `local.ItemIndex` _returnvalue)
  (`/Game/Gameplay/InventorySystem/ItemInterfaces/IBP_Item.SetCurrentInventory` _newitem null)
  ;[1 1 1] Add item widget to grid.
  (bind _itemwidget (`/Game/Gameplay/InventorySystem/ItemInterfaces/IBP_Item.GetItemWidget` (`local.NewItem`)))
  (bind _returnvalue_2 (`GridPanel.AddChildToGrid` (`self.GridPanelOfItems`) _itemwidget))
  (`GridSlot.SetColumn` _returnvalue_2 (mod _itemindex _inventorygridmaxcolumns))
  (`GridSlot.SetRow` _returnvalue_2 (/ _itemindex _inventorygridmaxcolumns)))

(fn `CountItem`
  (returns (ItemCount :type Integer))
  (return 0))

(fn `CountItems1`
  (returns (NumberOfItems :type Integer))
  (return (`KismetArrayLibrary.Array_Length` (`self.Items`))))

(fn `HideInventory`
  (if (`Widget.IsInViewport` (`self.InventoryWidget`))
    (`Widget.RemoveFromParent` (`self.InventoryWidget`))
    (else
      (`KismetSystemLibrary.PrintString` "Something has tried to call BP_MessengerInventory's HideInventory function, when WBP_Inventory is not in viewport!" true true (struct :`R` 1.0 :`G` 1.0 :`A` 1.0) 10.0))))

(fn `RemoveItem`
  (params (ItemToRemove :type "/Game/Gameplay/InventorySystem/ItemInterfaces/IBP_Item Interface"))
  (returns (Successful :type Boolean))
  (return false))

(fn `RemoveItem1`
  (params (ItemToRemove :type "/Game/Gameplay/InventorySystem/ItemInterfaces/IBP_Item Interface"))
  (bind _inventorygridmaxcolumns (`self.InventoryGridMaxColumns`))
  (bind _gridpanelofitems (`self.GridPanelOfItems`))
  (`|ExecutionSequence`
    (:`then_0`
      ;[1 1 1] Backend array removal
      (`KismetArrayLibrary.Array_RemoveItem` (`self.Items`) (`local.ItemToRemove`)))
    (:`then_1`
      ;[1 1 1] Clear the grid panel, then re-add, because grid panel's "Remove Child" seems broken.
      (`PanelWidget.ClearChildren` _gridpanelofitems)
      (for (_array_element _array_index) (`self.Items`)
        (bind _itemwidget (`/Game/Gameplay/InventorySystem/ItemInterfaces/IBP_Item.GetItemWidget` _array_element))
        (bind _returnvalue (`GridPanel.AddChildToGrid` _gridpanelofitems _itemwidget))
        (`GridSlot.SetColumn` _returnvalue (mod _array_index _inventorygridmaxcolumns))
        (`GridSlot.SetRow` _returnvalue (/ _array_index _inventorygridmaxcolumns))))))

(fn `SendItem`
  (params (ItemToSend :type "/Game/Gameplay/InventorySystem/ItemInterfaces/IBP_Item Interface"))
  ;[1 1 1] Is the owner BP_User in a waypoint?
  (bind _asbp_user (cast `/Game/Gameplay/BP_User` (`self.GetOwner`)))
  (bind _returnvalue (`E2EECharacter.GetCurrentWaypoint` _asbp_user))
  (if (`KismetSystemLibrary.IsValid` _returnvalue)
    ;[1 1 1] Is there a BP_Messenger in the waypoint?
    (for _array_element (`Waypoint.GetOccupants` _returnvalue)
      (cast `/Game/Gameplay/BP_Messenger` _array_element)
      ;[1 1 1] Send the item.
      (`self.RemoveItem` (`local.ItemToSend`))
      (`/Game/Gameplay/BP_Messenger.StartDeliverItem` (`self.TheMessenger`) (`local.ItemToSend`))
      (return)))
  ;[1 1 1] Conditions aren't met.
  (`/Game/Gameplay/BPFuncLib_Utilities.DisplayNotification` "Get close to the Messenger before sending items.")
  (return))

(fn `SetInventoryDimensions`
  (bind _returnvalue (`|CreateWidget` "/Game/UI/ItemWidgets/WBP_Lock.WBP_Lock_C"))
  (bind (_returnvalue_x _returnvalue_y) (`KismetMathLibrary.BreakVector2D` (/ (`CanvasPanelSlot.GetSize` (`WidgetLayoutLibrary.SlotAsCanvasSlot` (`self.GridPanelOfItems`))) (`.ImageSize` (break `SlateBrush` (`Image.Brush` (`/Game/UI/ItemWidgets/WBP_Lock.Image_Icon` _returnvalue)))))))
  (bind _output_get (set `self.InventoryGridMaxColumns` (`KismetMathLibrary.FTrunc` _returnvalue_x)))
  (bind _output_get_2 (set `self.InventoryGridMaxRows` (`KismetMathLibrary.FTrunc` _returnvalue_y)))
  (set `self.InventoryGridStoragePerPage` (* _output_get_2 _output_get)))

(fn `ShowInventory`
  (if (`Widget.IsInViewport` (`self.InventoryWidget`))
    (`KismetSystemLibrary.PrintString` "Something has tried to call BP_MessengerInventory's ShowInventory function, when WBP_Inventory is already in viewport!" true true (struct :`R` 1.0 :`G` 1.0 :`A` 1.0) 10.0)
    (else
      (`UserWidget.AddToViewport` (`self.InventoryWidget`) 0))))